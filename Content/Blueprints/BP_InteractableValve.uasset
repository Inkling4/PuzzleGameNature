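; BP_InteractableValve is an interactable valve that runs a countdown for a set active time once activated.
; BeginPlay caches the timer component's WBP_ValveTimerBar widget and sets its maximum time.
; ValveActivated resets the remaining time, which Tick counts down to zero and pushes to the widget each frame.
; Activation and disable events print debug messages, and nothing in these graphs fires the disable event on expiry.
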(event EventTick
  (params (DeltaSeconds :type Float%20%28single-precision%29))
  ;[0.15 0.15 0.15 0.5] Counts down the time in seconds, updates widget accordingly.
  (Utilities|FlowControl|Sequence
    (:then_0
      (Utilities|IsValid (Variables|Default|GetValveTimerRef)
        (:Is%20Valid
          ;;[0.15 0.15 0.15 0.5] This specific "Time remaining" variable in particular is the widget's variable, not this blueprint.
          (Variables|/Game/UI/WBP_ValveTimerBar.WBP_ValveTimerBar_C|SetTimeRemaining (Variables|Default|GetValveTimerRef) (Variables|Default|GetTimeRemaining)))))
    (:then_1
      (if (not (< (Variables|Default|GetTimeRemaining) 0.0))
        (bind _output_get (Variables|Default|SetTimeRemaining (- (Variables|Default|GetTimeRemaining) DeltaSeconds)))
        (if (< _output_get 0.0)
          (Variables|Default|SetTimeRemaining 0.0))))))

(event EventBeginPlay
  ;[0.15 0.15 0.15 0.5] Makes a class ref to the valve timer widget, and sets the max time.
  (bind _aswbp_valve_timer_bar (Utilities|Casting|CastToWBP_ValveTimerBar (UserInterface|GetWidget (Variables|Default|GetTimer))))
  (bind _output_get (Variables|Default|SetValveTimerRef _aswbp_valve_timer_bar))
  (Variables|/Game/UI/WBP_ValveTimerBar.WBP_ValveTimerBar_C|SetMaxTime _output_get (Variables|Default|GetActiveValveTime)))

(event EventValveActivated
  (Utilities|FlowControl|Sequence
    (:then_0
      (Variables|Default|SetTimeRemaining (Variables|Default|GetActiveValveTime)))
    (:then_1
      (Development|PrintString "Valve activated!" true true "(R=0.000000,G=0.797515,B=1.000000,A=1.000000)"))))

(event EventValveDisabled
  (Development|PrintString "Valve disabled!" true true "(R=1.000000,G=0.000000,B=0.000000,A=1.000000)"))

(fn ConstructionScript)