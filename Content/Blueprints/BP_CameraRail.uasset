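; BP_CameraRail is a camera rail actor that currently moves its camera through debug-key test input.
; Debug keys D and S set held flags, and Tick calls MoveCamera with a step of RailSpeed scaled by delta time, forward for D and backward for S.
; Disconnected, failed experiments to aim the camera at BP_Protagonist remain in the graph and never run.
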(event EventTick
  (params (DeltaSeconds :type Float%20%28single-precision%29))
  ;[0.15 0.15 0.15 0.5] Test to activate function "move camera"
  (if (Variables|Default|GetIs%20Debug%20Key%20D%20pressed)
    (Class|CameraRail|MoveCamera (stale Input|KeyboardEvents|DebugKeyD _output_get) (* DeltaSeconds (Variables|Default|GetRailSpeed)) :!label _label)
    (elif (Variables|Default|GetIs%20debug%20key%20S%20pressed)
      (goto _label))))

(event Collision|EventActorBeginOverlap
  (params (OtherActor :type Actor%20Object%20Reference)))

(event EventBeginPlay
  (Variables|Default|SetIs%20Debug%20Key%20D%20pressed false)
  (Variables|Default|SetIs%20debug%20key%20S%20pressed false))

(event Input|KeyboardEvents|DebugKeyS
  (params (Key :type Key%20Structure :default "None") (ActionValue :type Input%20Action%20Value%20Structure))
  ;[0.15 0.15 0.15 0.5] Test to activate function "move camera"
  (:Pressed
    (Variables|Default|SetIs%20debug%20key%20S%20pressed true))
  (:Released
    (Variables|Default|SetIs%20debug%20key%20S%20pressed false)))

(event Input|KeyboardEvents|DebugKeyD
  (params (Key :type Key%20Structure :default "None") (ActionValue :type Input%20Action%20Value%20Structure))
  ;[0.15 0.15 0.15 0.5] Test to activate function "move camera"
  (:Pressed
    (bind _output_get (Variables|Default|SetIs%20Debug%20Key%20D%20pressed true)))
  (:Released
    (Variables|Default|SetIs%20Debug%20Key%20D%20pressed false)))

(fn ConstructionScript)