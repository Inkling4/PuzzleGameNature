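; BP_BreakableGate is a gate actor that records its own destruction on the player character.
; When destroyed, it casts player controller 0's controlled pawn to BP_Protagonist and sets HasTheGateBeenBroken to true.
; It contains no breaking or damage logic of its own; the other default events are disabled and the construction script only calls its parent.
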(event EventBeginPlay
  (|CallParentFunction) ; This node is disabled and will not be called.\nDrag off pins to build functionality.
)

(event Collision|EventActorBeginOverlap
  (params (OtherActor :type Actor%20Object%20Reference))
  (|CallParentFunction OtherActor) ; This node is disabled and will not be called.\nDrag off pins to build functionality.
)

(event EventTick
  (params (DeltaSeconds :type Float%20%28single-precision%29))
  (|CallParentFunction DeltaSeconds) ; This node is disabled and will not be called.\nDrag off pins to build functionality.
)

(event EventOnDestroy
  (bind _asbp_protagonist (Utilities|Casting|CastToBP_Protagonist (Pawn|GetControlledPawn (Game|GetPlayerController 0))))
  (Variables|/Game/Blueprints/BP_Protagonist.BP_Protagonist_C|SetHasTheGateBeenBroken _asbp_protagonist true))

(fn ConstructionScript
  (|CallParentFunction))