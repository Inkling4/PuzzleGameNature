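; BP_NextLevelInteract is a Blueprint that handles moving the player to the next level.
; Its NextLevel event compares the current level name, converted to text, against hard-coded names: City opens Sewer, while the Sewer branch calls Open Level by Object Reference with no level assigned.
; BeginPlay, overlap, Tick and the construction script are empty, and nothing in this Blueprint calls NextLevel.
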(event EventBeginPlay)

(event Collision|EventActorBeginOverlap
  (params (OtherActor :type Actor%20Object%20Reference)))

(event EventTick
  (params (DeltaSeconds :type Float%20%28single-precision%29)))

(event EventNextLevel
  ;[0.15 0.15 0.15 0.5] Opens level based on current level name
  (bind _returnvalue (Game|GetCurrentLevelName true))
  (Variables|Default|SetCurrent%20Level%20Name (Utilities|Text|ToText(String) _returnvalue))
  (if (Utilities|Enum|Equal(Enum) (Variables|Default|GetCurrent%20Level%20Name) (Utilities|Text|ToText(String) "City"))
    (Game|OpenLevel(byObjectReference) "/Game/Maps/Sewer.Sewer")
    (elif (Utilities|Enum|Equal(Enum) (Variables|Default|GetCurrent%20Level%20Name) (Utilities|Text|ToText(String) "Sewer"))
      (Game|OpenLevel(byObjectReference)))))

(fn ConstructionScript)