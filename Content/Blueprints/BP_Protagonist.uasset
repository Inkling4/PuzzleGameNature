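; Player protagonist Blueprint that registers itself with the game instance and handles pausing.
; On BeginPlay it stores itself as PlayerCharacter in BP_GameInstance and, if the LoadGame flag is set, runs the load functions and clears the flag.
; The IA_Pause input opens WBP_PauseMenu, shows the cursor, switches to UI-only input and pauses the game.
; An unconnected snippet for switching the view to BP_CameraRail remains unused, as a separate camera actor is used.
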(event Input|EnhancedActionEvents|EnhancedInputActionIA_Pause
  (params (ActionValue :type Boolean) (ElapsedSeconds :type Float%20%28double-precision%29) (TriggeredSeconds :type Float%20%28double-precision%29) (InputAction :type Input%20Action%20Object%20Reference :default "/Game/Input/IA_Pause.IA_Pause"))
  (bind _returnvalue (Game|GetPlayerController 0))
  ;[0.15 0.15 0.15 0.5] Pause Function
  (:Started
    (bind _returnvalue_2 (Game|ConstructObjectfromClass "/Game/UI/WBP_PauseMenu.WBP_PauseMenu_C"))
    (UserInterface|Viewport|AddtoViewport _returnvalue_2 0)
    (Variables|/Script/Engine.PlayerController|SetbShowMouseCursor _returnvalue true)
    (Input|SetInputModeUIOnly _returnvalue 0 "DoNotLock" false)
    (Game|SetGamePaused true)))

(event Collision|EventActorBeginOverlap
  (params (OtherActor :type Actor%20Object%20Reference)))

(event EventTick
  (params (DeltaSeconds :type Float%20%28single-precision%29)))

(event EventBeginPlay
  (Utilities|FlowControl|Sequence
    (:then_1
      (bind _asbp_game_instance (Utilities|Casting|CastToBP_GameInstance (Game|GetGameInstance)))
      (bind _output_get (Variables|Default|SetGameInstanceReference _asbp_game_instance))
      (Variables|/Game/Blueprints/SaveGame/BP_GameInstance.BP_GameInstance_C|SetPlayerCharacter _output_get self)
      (if (Variables|/Game/Blueprints/SaveGame/BP_GameInstance.BP_GameInstance_C|GetLoadGame? (Variables|Default|GetGameInstanceReference))
        (Default|GameLoad (Variables|Default|GetGameInstanceReference))
        (Default|LoadGame (Variables|Default|GetGameInstanceReference))
        (Variables|/Game/Blueprints/SaveGame/BP_GameInstance.BP_GameInstance_C|SetLoadGame? (Variables|Default|GetGameInstanceReference) false)))))

(fn ConstructionScript)